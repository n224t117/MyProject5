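; BP_Dummy is a damageable dummy actor that tracks health and shows it on an HP bar widget.
; TakeDamageCustom subtracts damage from Health, clamps it between zero and MaxHealth, then passes the health ratio to the WBP_HPBar held by the HPBarWidget component.
; The event graph and construction script are empty, and the file contains no death handling.
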(fn `TakeDamageCustom`
  (params (Damage :type "Float (double-precision)"))
  (bind _health (`self.Health`))
  (set `self.Health` (`KismetMathLibrary.FClamp` (- _health Damage) 0.0 (`self.MaxHealth`)))
  (bind _aswbp_hpbar (cast `/Game/WBP_HPBar` (`WidgetComponent.GetUserWidgetObject` (`self.HPBarWidget`))))
  (`/Game/WBP_HPBar.SetHPPercent` _aswbp_hpbar (/ _health (`self.MaxHealth`))))

(fn `UserConstructionScript`)